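; BP_LaserBurst is a Gameplay Ability, apparently an unfinished laser burst attack: ActivateAbility has nothing connected, so it currently does nothing when activated.
; Disconnected draft chains build a BP_GE_Damage spec, setting Damage through the Effect.Damage SetByCaller tag.
; They try applying it either to an ability system component or to players at a grid cell from ANKGameState, with some ending the ability.
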(event Ability|EventActivateAbility)