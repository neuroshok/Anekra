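; Gameplay Cue that shows the Laser Burst ability's beam effect while the cue is active.
; WhileActive stores the instigator and attaches the FX_LaserBurst Niagara system to player 0's head socket, not the instigator's; OnRemove destroys it.
; Tick traces WorldDynamic objects from the instigator and feeds the hit, or its head socket if none, into the effect's TargetLocation.
; The camera-forward endpoint calculation is unconnected, so the trace end is unset.
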(event EventTick
  (params (DeltaSeconds :type Float%20%28single-precision%29))
  (if (Variables|Default|GetIsActive)
    (bind _outhit (Collision|LineTraceForObjects 0 (Transformation|GetActorLocation (Variables|Default|GetSource)) "0, 0, 0" (Utilities|Array|MakeArray (Utilities|Enum|LiteralenumEObjectTypeQuery "ObjectTypeQuery2")) false 0 "None"))
    (if (Math|Vector|VectorIsZero (.Location (Collision|BreakHitResult _outhit)))
      (Variables|Default|SetTargetLocation (Transformation|GetSocketLocation (Actor|GetComponentbyClass (Variables|Default|GetSource) "/Script/Engine.SkeletalMeshComponent") "head"))
      (else
        (Variables|Default|SetTargetLocation (.Location (Collision|BreakHitResult _outhit)))))
    (Niagara|SetNiagaraVariable(Vector3) (Variables|Default|GetFX) "TargetLocation" (Variables|Default|GetTargetLocation))))

(fn ConstructionScript)

(fn OnRemove
  (params (MyTarget :type Actor%20Object%20Reference) (Parameters :type Gameplay%20Cue%20Parameters%20Structure%20%28by%20ref%29))
  (Variables|Default|SetIsActive false)
  (Components|DestroyComponent (Variables|Default|GetFX))
  (return false))

(fn WhileActive
  (params (MyTarget :type Actor%20Object%20Reference) (Parameters :type Gameplay%20Cue%20Parameters%20Structure%20%28by%20ref%29))
  (Variables|Default|SetSource (Class|AbilitySystemBlueprintLibrary|EffectContextGetInstigatorActor (.EffectContext (Ability|GameplayCue|BreakGameplayCueParameters Parameters))))
  (Variables|Default|SetIsActive true)
  (Variables|Default|SetCueParameters "")
  (bind _returnvalue (Niagara|SpawnSystemAttached "/Game/anekra/ability/laserburst/FX_LaserBurst.FX_LaserBurst" (Actor|GetComponentbyClass (Game|Player|GetPlayerPawn 0) "/Script/Engine.SkeletalMeshComponent") "head" "0, 0, 0" "0, 0, 0" "KeepRelativeOffset" false))
  (Variables|Default|SetFX _returnvalue)
  (return false))