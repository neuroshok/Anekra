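; Gameplay Cue notify actor for an unlock effect, showing a Niagara system while the cue is active.
; OnActive spawns the unlock system attached to the cue's own scene root and stores it as FX.
; OnRemove calls DestroyComponent on player 0's pawn root component, passing FX as the argument rather than targeting FX itself.
; Both handlers return false, and the event graph and construction script are empty.
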(event EventBeginPlay)

(event Collision|EventActorBeginOverlap
  (params (OtherActor :type Actor%20Object%20Reference)))

(event EventTick
  (params (DeltaSeconds :type Float%20%28single-precision%29)))

(fn ConstructionScript)

(fn OnRemove
  (params (MyTarget :type Actor%20Object%20Reference) (Parameters :type Gameplay%20Cue%20Parameters%20Structure%20%28by%20ref%29))
  (Components|DestroyComponent (Variables|/Script/Engine.Actor|GetRootComponent (Game|Player|GetPlayerPawn 0)) (Variables|Default|GetFX))
  (return false))

(fn OnActive
  (params (MyTarget :type Actor%20Object%20Reference) (Parameters :type Gameplay%20Cue%20Parameters%20Structure%20%28by%20ref%29))
  (bind _returnvalue (Niagara|SpawnSystemAttached "/Game/fx/FX_Unlock_System.FX_Unlock_System" (Variables|Default|GetDefaultSceneRoot) "None" "0, 0, 0" "0, 0, 0" "KeepRelativeOffset" false))
  (Variables|Default|SetFX _returnvalue)
  (return false))